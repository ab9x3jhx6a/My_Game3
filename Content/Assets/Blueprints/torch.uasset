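; A torch Blueprint whose bounce and point lights dim over time and can be relit with the R key.
; BeginPlay stores the bounce light's starting intensity and enables player input, and pressing R sets both lights to that stored value.
; Tick lowers both lights by a fixed per-frame step, not scaled by delta time, while the bounce light is above a floor, otherwise re-enabling input.
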(event `Key|R`
  (params (Key :type "Key Structure" :default "AnyKey"))
  (bind _intensitystart (`self.IntensityStart`))
  (:`Pressed`
    (`LightComponent.SetIntensity` (`self.BounceLight`) _intensitystart)
    (`LightComponent.SetIntensity` (`self.PointLight`) _intensitystart)))

(event `self.ReceiveBeginPlay`
  (set `self.IntensityStart` (`LightComponentBase.Intensity` (`self.BounceLight`)))
  (`self.EnableInput` (`GameplayStatics.GetPlayerController` 0) :!label _label))

(event `self.ReceiveTick`
  (params (DeltaSeconds :type "Float (single-precision)"))
  (bind _bouncelight (`self.BounceLight`))
  (bind _pointlight (`self.PointLight`))
  (bind _intensity (`LightComponentBase.Intensity` _bouncelight))
  (if (> _intensity 1000.0)
    (`LightComponent.SetIntensity` _bouncelight (- _intensity 50.0))
    (`LightComponent.SetIntensity` _pointlight (- (`LightComponentBase.Intensity` _pointlight) 50.0))
    (else
      (goto _label))))

(fn `UserConstructionScript`)